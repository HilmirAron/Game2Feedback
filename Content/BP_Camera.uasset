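; BP_Camera is the player's camera pawn for a game built around six doors bound to the S, D, F, J, K and L keys.
; Pressing a key calls ToggleDoor with false on that key's door, but only if the door is occupied.
; On BeginPlay it creates the UI_Score widget, passes itself as the pawn reference and adds it to the viewport.
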(event EventBeginPlay
  (bind _returnvalue (UserInterface|CreateWidget "/Game/UI_Score.UI_Score_C" 0 self))
  (UserInterface|Viewport|AddtoViewport _returnvalue 0))

(event Input|KeyboardEvents|K
  (params (Key :type Key%20Structure :default "None"))
  (bind _doork (Variables|Default|GetDoorK))
  (:Pressed
    (if (Variables|/Game/bp_door.bp_door_C|GetOccupied _doork)
      (Default|ToggleDoor _doork false))))

(event Input|KeyboardEvents|L
  (params (Key :type Key%20Structure :default "None"))
  (bind _doorl (Variables|Default|GetDoorL))
  (:Pressed
    (if (Variables|/Game/bp_door.bp_door_C|GetOccupied _doorl)
      (Default|ToggleDoor _doorl false))))

(event Input|KeyboardEvents|D
  (params (Key :type Key%20Structure :default "None"))
  (bind _doord (Variables|Default|GetDoorD))
  (:Pressed
    (if (Variables|/Game/bp_door.bp_door_C|GetOccupied _doord)
      (Default|ToggleDoor _doord false))))

(event Input|KeyboardEvents|S
  (params (Key :type Key%20Structure :default "None"))
  (bind _doors (Variables|Default|GetDoorS))
  (:Pressed
    (if (Variables|/Game/bp_door.bp_door_C|GetOccupied _doors)
      (Default|ToggleDoor _doors false))))

(event Input|KeyboardEvents|J
  (params (Key :type Key%20Structure :default "None"))
  (bind _doorj (Variables|Default|GetDoorJ))
  (:Pressed
    (if (Variables|/Game/bp_door.bp_door_C|GetOccupied _doorj)
      (Default|ToggleDoor _doorj false))))

(event Input|KeyboardEvents|F
  (params (Key :type Key%20Structure :default "None"))
  (bind _doorf (Variables|Default|GetDoorF))
  (:Pressed
    (if (Variables|/Game/bp_door.bp_door_C|GetOccupied _doorf)
      (Default|ToggleDoor _doorf false))))

(fn ConstructionScript)