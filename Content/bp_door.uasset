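; Door actor that periodically spawns a BP_Visitor guest and swings open when one appears.
; After a short random delay at BeginPlay, SpawnGuest places the visitor at an offset, passes it a door reference, opens the door and marks it occupied.
; ToggleDoor snaps the door's rotation; closing it destroys any valid visitor and schedules the next spawn after a random delay.
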(event Custom|ToggleDoor
  (params (Open :type Boolean))
  (bind _myvisitor (Variables|Default|GetMyVisitor))
  (if Open
    (Transformation|SetRelativeRotation (Variables|Default|GetDoor) "0.000000,-120.000000,0.000000" false false)
    (else
      (Transformation|SetRelativeRotation (Variables|Default|GetDoor) "0.000000,0.000000,0.000000" false false)
      (Utilities|IsValid _myvisitor
        (:Is%20Valid
          (Actor|DestroyActor _myvisitor)
          (Utilities|FlowControl|Delay (Math|Random|RandomFloatinRange 3.0 15.0))
          (CallFunction|SpawnGuest))))))

(event Custom|SpawnGuest
  (bind _returnvalue (Transformation|GetActorTransform))
  (bind _returnvalue_2 (Game|SpawnActorfromClass "/Game/BP_Visitor.BP_Visitor_C" (Math|Transform|MakeTransform (+ (.location _returnvalue) "-50.000000,-75.000000,0.000000") (Math|Rotator|MakeRotator (.roll (.rotation _returnvalue)) (.pitch (.rotation _returnvalue)) (+ (.yaw (.rotation _returnvalue)) 9e+01)) (.scale _returnvalue)) "Undefined" "MultiplyWithRoot" 0 self 0))
  (Variables|Default|SetMyVisitor _returnvalue_2)
  (CallFunction|ToggleDoor true)
  (Variables|Default|SetOccupied true))

(event EventBeginPlay
  (Utilities|FlowControl|Delay (Math|Random|RandomFloatinRange 1.0 5.0))
  (CallFunction|SpawnGuest))

(fn ConstructionScript)