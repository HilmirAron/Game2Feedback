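; BP_Visitor is a guest actor tied to a door that randomly spawns as a good or bad visitor and affects the player's money.
; BeginPlay flips a random bool to set IaMBad and the matching skeletal mesh materials, then waits briefly before calling TriggerGuest.
; TriggerGuest deducts money from the BP_Camera player pawn for bad guests or adds it for good ones, then calls ToggleDoor(false) on MyDoor and destroys itself.
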(event Custom|TriggerGuest
  (if (Variables|Default|GetIaMBad)
    (bind _asbp_camera (Utilities|Casting|CastToBP_Camera (Game|Player|GetPlayerPawn 0)))
    (Variables|/Game/BP_Camera.BP_Camera_C|SetMoney _asbp_camera (+ (Variables|/Game/BP_Camera.BP_Camera_C|GetMoney _asbp_camera) -30))
    (else
      (bind _asbp_camera_2 (Utilities|Casting|CastToBP_Camera (Game|Player|GetPlayerPawn 0)))
      (Variables|/Game/BP_Camera.BP_Camera_C|SetMoney _asbp_camera_2 (+ (Variables|/Game/BP_Camera.BP_Camera_C|GetMoney _asbp_camera_2) 10))))
  (Default|ToggleDoor (Variables|Default|GetMyDoor) false)
  (Actor|DestroyActor))

(event EventBeginPlay
  (if (Math|Random|RandomBool)
    (Variables|Default|SetIaMBad true)
    (Rendering|Material|SetMaterial (Variables|Default|GetSkeletalMesh) 0 "/Game/mat_badguy.mat_badguy")
    (Rendering|Material|SetMaterial (Variables|Default|GetSkeletalMesh) 1 "/Game/mat_badguy.mat_badguy")
    (else
      (Variables|Default|SetIaMBad false)
      (Rendering|Material|SetMaterial (Variables|Default|GetSkeletalMesh) 0 "/Game/mat_goodGuy.mat_goodGuy")
      (Rendering|Material|SetMaterial (Variables|Default|GetSkeletalMesh) 1 "/Game/mat_goodGuy.mat_goodGuy")))
  (Utilities|FlowControl|Delay 2.0)
  (CallFunction|TriggerGuest))

(fn ConstructionScript)